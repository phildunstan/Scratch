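; BP_ScatchCharacter is a character Blueprint that turns Enhanced Input actions into movement relative to the actor's own rotation.
; Four directional actions scale the actor's forward or right vector by the action value, negated for backward and left.
; IA_Move combines both axes from a single action value, with X as right and Y as forward.
; Every handler feeds its vector straight into CharacterMovement through AddInputVector.
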(event `EnhancedInput|/Game/Input/IA_Forward`
  (params (ActionValue :type "Float (double-precision)") (ElapsedSeconds :type "Float (double-precision)") (TriggeredSeconds :type "Float (double-precision)") (InputAction :type "InputAction Object Reference" :default "/Game/Input/IA_Forward.IA_Forward"))
  (:`Triggered`
    (`PawnMovementComponent.AddInputVector` (`self.CharacterMovement`) (* ActionValue (`KismetMathLibrary.GetForwardVector` (`self.K2_GetActorRotation`))) false)))

(event `EnhancedInput|/Game/Input/IA_Backward`
  (params (ActionValue :type "Float (double-precision)") (ElapsedSeconds :type "Float (double-precision)") (TriggeredSeconds :type "Float (double-precision)") (InputAction :type "InputAction Object Reference" :default "/Game/Input/IA_Backward.IA_Backward"))
  (:`Triggered`
    (`PawnMovementComponent.AddInputVector` (`self.CharacterMovement`) (* (* ActionValue -1.0) (`KismetMathLibrary.GetForwardVector` (`self.K2_GetActorRotation`))) false)))

(event `EnhancedInput|/Game/Input/IA_Right`
  (params (ActionValue :type "Float (double-precision)") (ElapsedSeconds :type "Float (double-precision)") (TriggeredSeconds :type "Float (double-precision)") (InputAction :type "InputAction Object Reference" :default "/Game/Input/IA_Right.IA_Right"))
  (:`Triggered`
    (`PawnMovementComponent.AddInputVector` (`self.CharacterMovement`) (* ActionValue (`KismetMathLibrary.GetRightVector` (`self.K2_GetActorRotation`))) false)))

(event `EnhancedInput|/Game/Input/IA_Left`
  (params (ActionValue :type "Float (double-precision)") (ElapsedSeconds :type "Float (double-precision)") (TriggeredSeconds :type "Float (double-precision)") (InputAction :type "InputAction Object Reference" :default "/Game/Input/IA_Left.IA_Left"))
  (:`Triggered`
    (`PawnMovementComponent.AddInputVector` (`self.CharacterMovement`) (* (* ActionValue -1.0) (`KismetMathLibrary.GetRightVector` (`self.K2_GetActorRotation`))) false)))

(event `EnhancedInput|/Game/Input/IA_Move`
  (params (ActionValue :type "Vector2D Structure") (ElapsedSeconds :type "Float (double-precision)") (TriggeredSeconds :type "Float (double-precision)") (InputAction :type "InputAction Object Reference" :default "/Game/Input/IA_Move.IA_Move"))
  (:`Triggered`
    (`PawnMovementComponent.AddInputVector` (`self.CharacterMovement`) (+ (* ActionValue_X (`KismetMathLibrary.GetRightVector` (`self.K2_GetActorRotation`))) (* ActionValue_Y (`KismetMathLibrary.GetForwardVector` (`self.K2_GetActorRotation`)))) false)))

(fn `UserConstructionScript`)